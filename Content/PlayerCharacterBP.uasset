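; Player character Blueprint with axis-driven movement and look, plus overlap-triggered NPC conversations shown in a DialogHUD widget alongside money.
; Overlapping an NPCPawnBP loads its dialog, while ending any overlap clears it.
; DialogCase is a semicolon-delimited string of question, options and next-dialog indices, which button events follow.
; Tick updates debug text and polls DialogUpdated; overlapping AgilityAIController-driven PathCharacterBPs flags them to move on.
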(event `self.ReceiveBeginPlay`
  (bind _returnvalue (`GameplayStatics.GetPlayerController` 0))
  (`|ExecutionSequence`
    (:`then_0`
      (`WidgetBlueprintLibrary.SetInputMode_GameAndUIEx` _returnvalue null)
      (set `PlayerController.bShowMouseCursor` true _returnvalue))
    (:`then_1`
      (bind _returnvalue_2 (`|CreateWidget` "/Game/DialogHUD.DialogHUD_C"))
      (bind _output_get (set `self.DialogHUD` _returnvalue_2))
      (`UserWidget.AddToViewport` _output_get 0))
    (:`then_2`
      (add `self.UpdateDialogED` (delegate `UpdateDialogHUDEvent`)))))

(event `UpdateDialogHUDEvent` :!signature `self.UpdateDialogED`
  (params (DialogBtn :type Integer))
  (bind _dialoghud (`self.DialogHUD`))
  (bind _returnvalue (`KismetStringLibrary.ParseIntoArray` (`self.DialogCase`) ";"))
  (switch `int` DialogBtn
    (:`0`
      (`self.NextDialog` (`KismetStringLibrary.Conv_StringToInt` (`|GetArrayItem` _returnvalue 2))))
    (:`1`
      (`self.NextDialog` (`KismetStringLibrary.Conv_StringToInt` (`|GetArrayItem` _returnvalue 4))))
    (:`2`
      (`self.NextDialog` (`KismetStringLibrary.Conv_StringToInt` (`|GetArrayItem` _returnvalue 6)))))
  (for _array_element (`NPCPawn.ShortMemory` (`self.TalkNPC`))
    (`KismetSystemLibrary.PrintString` (`KismetStringLibrary.Conv_IntToString` _array_element)))
  (`TextBlock.SetText` (`/Game/DialogHUD.DialogQuestion` _dialoghud) (`KismetTextLibrary.Conv_StringToText` (`|GetArrayItem` _returnvalue)) :!label _label)
  (`TextBlock.SetText` (`/Game/DialogHUD.opt1text` _dialoghud) (`KismetTextLibrary.Conv_StringToText` (`|GetArrayItem` _returnvalue 1)))
  (`TextBlock.SetText` (`/Game/DialogHUD.opt2text` _dialoghud) (`KismetTextLibrary.Conv_StringToText` (`|GetArrayItem` _returnvalue 3)))
  (`TextBlock.SetText` (`/Game/DialogHUD.opt3text` _dialoghud) (`KismetTextLibrary.Conv_StringToText` (`|GetArrayItem` _returnvalue 5))))

(event `self.ReceiveTick`
  (params (DeltaSeconds :type "Float (single-precision)"))
  (bind _dialogcase (`self.DialogCase`))
  (`|ExecutionSequence`
    (:`then_0`
      ;[1 1 1] DEBUG current dialog case
      (`TextBlock.SetText` (`/Game/DialogHUD.CurrentDialogCase` (`self.DialogHUD`)) (`KismetTextLibrary.Conv_StringToText` (`KismetStringLibrary.Concat_StrStr` (`KismetStringLibrary.Conv_IntToString` (`KismetArrayLibrary.Array_Length` (`KismetStringLibrary.ParseIntoArray` _dialogcase ";"))) _dialogcase))))
    (:`then_1`
      ;[1 1 1] Mäkkaiver
      (if (`self.DialogUpdated`)
        (if (> (`KismetArrayLibrary.Array_Length` (`KismetStringLibrary.ParseIntoArray` (`self.DialogCase`) ";")) 1) :!label _label_2
          (goto _label)
          (else
            (goto _label)))))
    (:`then_2`
      (`TextBlock.SetText` (`/Game/DialogHUD.MoneyField` (`self.DialogHUD`)) (`KismetTextLibrary.Conv_StringToText` (`KismetStringLibrary.Concat_StrStr` "Money: " (`KismetStringLibrary.Conv_DoubleToString` (`self.Money`))))))))

(event `self.DialogCollision.OnComponentBeginOverlap`
  (params (OverlappedComponent :type "PrimitiveComponent Object Reference") (OtherActor :type "Actor Object Reference") (OtherComp :type "PrimitiveComponent Object Reference") (OtherBodyIndex :type Integer) (bFromSweep :type Boolean) (SweepResult :type "HitResult Structure (by ref)"))
  (bind _asnpcpawn_bp (cast `/Game/NPCPawnBP` OtherActor)
    (:`then`
      (bind _output_get (set `self.TalkNPC` _asnpcpawn_bp))
      (`self.UpdateDialogHUD` _output_get)
      (goto _label_2))
    (:`CastFailed`
      (bind _aspath_character_bp (cast `/Game/PathCharacterBP` OtherActor))
      (bind _asagility_aicontroller (cast `/Game/AgilityAIController` (`self.GetController` _aspath_character_bp)))
      (set `/Game/AgilityAIController.MoveToNext` true _asagility_aicontroller)
      (`SceneComponent.K2_SetWorldRotation` :`self` (`Actor.RootComponent` _aspath_character_bp)))))

(event `self.ReceiveActorEndOverlap`
  (params (OtherActor :type "Actor Object Reference"))
  (`self.EmptyDialogHUD`)
  (set `self.TalkNPC` null)
  (goto _label_2))

(event `InputAxis|MoveForward`
  (params (AxisValue :type "Float (single-precision)"))
  (`self.AddMovementInput` (`self.GetActorForwardVector`) AxisValue))

(event `InputAxis|VerticalLook`
  (params (AxisValue :type "Float (single-precision)"))
  (`self.AddControllerPitchInput` (* AxisValue -1.0)))

(event `InputAxis|MoveRight`
  (params (AxisValue :type "Float (single-precision)"))
  (`self.AddMovementInput` (`self.GetActorRightVector`) AxisValue))

(event `InputAxis|HorizontalLook`
  (params (AxisValue :type "Float (single-precision)"))
  (`self.AddControllerYawInput` AxisValue))

(fn `UserConstructionScript`)