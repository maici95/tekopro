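; NPC pawn that displays its name and what it holds about the player on floating text tags.
; BeginPlay sets the NPC name tag.
; Every Tick copies the player controller's rotation to all four tags with a 180-degree turn, and refreshes player name, intention and attitude text.
; Attitude is the sum of ShortMemory entries divided by MemorySize, recomputed each frame.
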(event `self.ReceiveBeginPlay`
  (`|ExecutionSequence`
    (:`then_0`
      (`TextRenderComponent.K2_SetText` (`self.NPCNameTag`) (`self.NPCName`)))))

(event `self.ReceiveTick`
  (params (DeltaSeconds :type "Float (single-precision)"))
  (bind _playernametag (`self.PlayerNameTag`))
  (bind _playerintentiontag (`self.PlayerIntentionTag`))
  (bind _attitudeperc (`self.AttitudePerc`))
  (bind _npcnametag (`self.NPCNameTag`))
  (bind _rotation (.rotation (`self.GetTransform` (`GameplayStatics.GetPlayerController` 0))))
  (`|ExecutionSequence`
    (:`then_0`
      (`SceneComponent.K2_SetWorldRotation` _npcnametag _rotation false false)
      (`SceneComponent.K2_AddLocalRotation` _npcnametag (struct :`Yaw` 180.0) false false))
    (:`then_1`
      (`SceneComponent.K2_SetWorldRotation` _playernametag _rotation false false)
      (`SceneComponent.K2_AddLocalRotation` _playernametag (struct :`Yaw` 180.0) false false))
    (:`then_2`
      (`SceneComponent.K2_SetWorldRotation` _playerintentiontag _rotation false false)
      (`SceneComponent.K2_AddLocalRotation` _playerintentiontag (struct :`Yaw` 180.0) false false))
    (:`then_3`
      (`TextRenderComponent.K2_SetText` _playernametag (`KismetTextLibrary.Conv_StringToText` (`KismetStringLibrary.Concat_StrStr` "Player name: " (`self.PlayerName`)))))
    (:`then_4`
      (`TextRenderComponent.K2_SetText` _playerintentiontag (`KismetTextLibrary.Conv_StringToText` (`KismetStringLibrary.Concat_StrStr` "Player intention: " (`self.PlayerIntention`))))
      (set `self.Attitude` 0.0)
      (for _array_element (`self.ShortMemory`)
        (bind _output_get (set `self.Attitude` (+ (`self.Attitude`) (`KismetMathLibrary.Conv_IntToDouble` _array_element)))))
      (`TextRenderComponent.K2_SetText` _attitudeperc (`KismetTextLibrary.Conv_StringToText` (`KismetStringLibrary.Concat_StrStr` "Player attitude: " (`KismetStringLibrary.Conv_DoubleToString` (/ _output_get (`KismetMathLibrary.Conv_IntToDouble` (`self.MemorySize`))))))))
    (:`then_5`
      (`SceneComponent.K2_SetWorldRotation` _attitudeperc _rotation false false)
      (`SceneComponent.K2_AddLocalRotation` _attitudeperc (struct :`Yaw` 180.0) false false))))

(fn `UserConstructionScript`)