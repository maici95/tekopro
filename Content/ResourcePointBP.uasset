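; ResourcePointBP is a resource point holding an amount that regrows over time, capped between fixed limits.
; Each Tick adds RegrowRate to ResAmount without delta-time scaling, so regrowth speed depends on frame rate.
; Two text renders display ResAmount and HasCollector, re-oriented every frame from the player controller's rotation with a half-turn flip.
; Nothing in this graph consumes the resource or sets HasCollector.
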(event `self.ReceiveTick`
  (params (DeltaSeconds :type "Float (single-precision)"))
  (bind _textrender (`self.TextRender`))
  (bind _textrender1 (`self.TextRender1`))
  (bind _rotation (.rotation (`self.GetTransform` (`GameplayStatics.GetPlayerController` 0))))
  (`|ExecutionSequence`
    (:`then_0`
      (`SceneComponent.K2_SetWorldRotation` _textrender _rotation false false)
      (`SceneComponent.K2_AddLocalRotation` _textrender (struct :`Yaw` 180.0) false false)
      (`TextRenderComponent.K2_SetText` _textrender (`KismetTextLibrary.Conv_DoubleToText` (`self.ResAmount`) "HalfToEven")))
    (:`then_1`
      (set `self.ResAmount` (`KismetMathLibrary.FClamp` (+ (`self.ResAmount`) (`self.RegrowRate`)) 0.0 100.0)))
    (:`then_2`
      (`SceneComponent.K2_SetWorldRotation` _textrender1 _rotation false false)
      (`SceneComponent.K2_AddLocalRotation` _textrender1 (struct :`Yaw` 180.0) false false)
      (`TextRenderComponent.K2_SetText` _textrender1 (`KismetTextLibrary.Conv_BoolToText` (`self.HasCollector`))))))

(fn `UserConstructionScript`)